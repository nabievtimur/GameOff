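; One-shot story trigger for the "First Contact" beat in MoonShot.
; When the player pawn overlaps its static mesh, it pauses the game, shows an ImagePrinter widget on top of the viewport and destroys itself.
; It also sets FirstContactDestroyed on GlobalVars_GameInstance to record the event.
; Tick checks WelcomeMessageDestroyed on that game instance but only calls the parent construction script, so it does not gate the trigger.
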(event OnComponentBeginOverlap(StaticMeshComponent)
  (params (OverlappedComponent :type Primitive%20Component%20Object%20Reference) (OtherActor :type Actor%20Object%20Reference) (OtherComp :type Primitive%20Component%20Object%20Reference) (OtherBodyIndex :type Integer) (bFromSweep :type Boolean) (SweepResult :type Hit%20Result%20Structure%20%28by%20ref%29))
  ;[1 1 1] Image Printer
  (if (== OtherActor (Game|Player|GetPlayerPawn 0))
    (Game|SetGamePaused true)
    ;;[0.4597 0.1188 1] ImageInput
    (bind _returnvalue (Game|ConstructObjectfromClass "/Game/MoonShot_TheGame_Custom_Files/StoryImages/ImagePrinter.ImagePrinter_C" (Game|GetPlayerController 0)))
    (UserInterface|Viewport|AddtoViewport _returnvalue 1000)
    (Actor|DestroyActor)
    (Variables|/Game/MoonShot_TheGame_Custom_Files/Maps/GlobalVars_GameInstance.GlobalVars_GameInstance_C|SetFirstContact_Destroyed (.AsGlobal%20Vars%20Game%20Instance (Utilities|Casting|CastToGlobalVars_GameInstance (Game|GetGameInstance))) true)
    (Development|PrintString "First Contact Destroyed")))

(event EventBeginPlay)

(event Collision|EventActorBeginOverlap
  (params (OtherActor :type Actor%20Object%20Reference))
  (|CallParentFunction OtherActor) ; This node is disabled and will not be called.\nDrag off pins to build functionality.
)

(event EventTick
  (params (DeltaSeconds :type Float%20%28single-precision%29))
  (if (Variables|/Game/MoonShot_TheGame_Custom_Files/Maps/GlobalVars_GameInstance.GlobalVars_GameInstance_C|GetWelcome_Message_Destroyed (.AsGlobal%20Vars%20Game%20Instance (Utilities|Casting|CastToGlobalVars_GameInstance (Game|GetGameInstance))))
    (|CallParentFunction)))

(fn ConstructionScript
  (|CallParentFunction))