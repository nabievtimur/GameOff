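; BP_DefaultEnemy_BossChild is a boss enemy variant that inherits its behavior from a parent enemy Blueprint.
; SetHealth fills CurrentHealth from MaxHealth, then starts a looping short-interval timer that calls Death by name and stores its handle in Timer.
; Death and the construction script only call their parent versions, and the event graph holds only disabled placeholder events.
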(event EventBeginPlay
  (|CallParentFunction) ; This node is disabled and will not be called.\nDrag off pins to build functionality.
)

(event Collision|EventActorBeginOverlap
  (params (OtherActor :type Actor%20Object%20Reference)))

(event EventTick
  (params (DeltaSeconds :type Float%20%28single-precision%29))
  (|CallParentFunction DeltaSeconds) ; This node is disabled and will not be called.\nDrag off pins to build functionality.
)

(fn ConstructionScript
  (|CallParentFunction))

(fn Death
  (|CallParentFunction))

(fn SetHealth
  (Variables|Default|SetCurrentHealth (Variables|Default|GetMaxHealth))
  (bind _returnvalue (Utilities|Time|SetTimerbyFunctionName 0 "Death" 0.1 true))
  (Variables|Default|SetTimer _returnvalue))