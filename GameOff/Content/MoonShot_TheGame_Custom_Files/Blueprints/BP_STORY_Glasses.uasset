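; BP_STORY_Glasses is a story pickup actor, apparently glasses, that shows an image screen when the player touches it.
; An overlap on its static mesh checks for the player pawn, pauses the game and adds an ImagePrinter_2 widget to the viewport at a high Z-order.
; The actor then destroys itself, so it triggers once, and nothing here unpauses the game.
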(event OnComponentBeginOverlap(StaticMeshComponent)
  (params (OverlappedComponent :type Primitive%20Component%20Object%20Reference) (OtherActor :type Actor%20Object%20Reference) (OtherComp :type Primitive%20Component%20Object%20Reference) (OtherBodyIndex :type Integer) (bFromSweep :type Boolean) (SweepResult :type Hit%20Result%20Structure%20%28by%20ref%29))
  ;[1 1 1] Image Printer
  (if (== OtherActor (Game|Player|GetPlayerPawn 0))
    (Game|SetGamePaused true)
    ;;[0.4597 0.1188 1] ImageInput
    (bind _returnvalue (Game|ConstructObjectfromClass "/Game/MoonShot_TheGame_Custom_Files/StoryImages/ImagePrinter_2.ImagePrinter_2_C" (Game|GetPlayerController 0)))
    (UserInterface|Viewport|AddtoViewport _returnvalue 1000)
    (Actor|DestroyActor)))

(event EventBeginPlay
  (|CallParentFunction) ; This node is disabled and will not be called.\nDrag off pins to build functionality.
)

(event Collision|EventActorBeginOverlap
  (params (OtherActor :type Actor%20Object%20Reference))
  (|CallParentFunction OtherActor) ; This node is disabled and will not be called.\nDrag off pins to build functionality.
)

(event EventTick
  (params (DeltaSeconds :type Float%20%28single-precision%29))
  (|CallParentFunction DeltaSeconds) ; This node is disabled and will not be called.\nDrag off pins to build functionality.
)

(fn ConstructionScript
  (|CallParentFunction))